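; BP_Button is a usable toggle button that shows its On or Off state on a text render component.
; BeginPlay sets the label from the initial IsButtonOn value.
; The BIUse event flips IsButtonOn, updates the label, then calls the ButtonPressed dispatcher with the new state.
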(event `self.ReceiveBeginPlay`
  (if (`self.isButtonOn`)
    (`TextRenderComponent.K2_SetText` (`self.TextRender`) (`KismetTextLibrary.Conv_StringToText` "On"))
    (else
      (`TextRenderComponent.K2_SetText` (`self.TextRender`) (`KismetTextLibrary.Conv_StringToText` "Off")))))

(event `/Game/MyHorror/Blueprints/UseInterface.BI_Use`
  (params (hitComponent :type "PrimitiveComponent Object Reference"))
  (bind _output_get (set `self.isButtonOn` (not (`self.isButtonOn`))))
  (if _output_get
    (`TextRenderComponent.K2_SetText` (`self.TextRender`) (`KismetTextLibrary.Conv_StringToText` "On"))
    (else
      (`TextRenderComponent.K2_SetText` (`self.TextRender`) (`KismetTextLibrary.Conv_StringToText` "Off"))))
  (`self.buttonPressed` (`self.isButtonOn`)))

(fn `UserConstructionScript`)