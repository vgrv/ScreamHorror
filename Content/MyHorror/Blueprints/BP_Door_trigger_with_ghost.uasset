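; Horror door trigger that, on first overlap, swings a door open and sends a ghost mesh gliding past.
; The OpenDoor timeline rotates the Arrow pivot; when finished, it reveals StaticMesh and starts Timeline_0 to slide it sideways.
; That slide blackens the mesh and immediately reverses the door once, whose finish re-triggers the slide from the mesh's current location.
; CanBeOpened checks the player's Keys for this door but is unused here.
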(event `self.Box.OnComponentBeginOverlap`
  (params (OverlappedComponent :type "PrimitiveComponent Object Reference") (OtherActor :type "Actor Object Reference") (OtherComp :type "PrimitiveComponent Object Reference") (OtherBodyIndex :type Integer) (bFromSweep :type Boolean) (SweepResult :type "HitResult Structure (by ref)"))
  (bind _initlocation (`self.initLocation`))
  (bind _staticmesh (`self.StaticMesh`))
  (`/Engine/EditorBlueprintResources/StandardMacros.DoOnce` false
    (:`Completed`
      (bind (_direction _dooropen) (`Timeline|OpenDoor` :!label _label)
        (:`Update`
          (`SceneComponent.K2_SetRelativeRotation` (`self.Arrow`) (`KismetMathLibrary.RLerp` (struct) (struct :`Yaw` -80.0) _dooropen) false false))
        (:`Finished`
          (`SceneComponent.SetVisibility` _staticmesh true false)
          (set `self.initLocation` (`SceneComponent.RelativeLocation` _staticmesh))
          (bind (_direction_2 _newtrack_4) (`Timeline|Timeline_0` :!via `PlayFromStart`)
            (:`Update`
              (`SceneComponent.K2_SetRelativeLocation` _staticmesh (`KismetMathLibrary.VLerp` _initlocation (+ _initlocation (0.0 -1200.0 0.0)) _newtrack_4) false false)
              (if true
                (`PrimitiveComponent.SetMaterial` _staticmesh 0 "/Game/BLACK.BLACK")
                (if true
                  (`/Engine/EditorBlueprintResources/StandardMacros.DoOnce` false
                    (:`Completed`
                      (goto _label :!via `ReverseFromEnd`))))))))))))

(fn `canBeOpened`
  (returns (canBeOpened :type Boolean))
  (bind _asfirst_person_character (cast `/Game/FirstPersonBP/Blueprints/FirstPersonCharacter` (`GameplayStatics.GetPlayerCharacter` 0)))
  (for _array_element (`/Game/FirstPersonBP/Blueprints/FirstPersonCharacter.keys` _asfirst_person_character)
    (if (== _array_element self)
      (return true)))
  (return false))

(fn `UserConstructionScript`)