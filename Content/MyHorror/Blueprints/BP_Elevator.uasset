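; BP_Elevator is an elevator actor that moves between placed target points when its floor buttons are used.
; The construction script stacks a numbered cube button above the Arrow for each entry in Targets.
; BIUse maps the hit button to its target by array index, ignoring presses while moving.
; A timeline lerps the whole actor transform to that target, with a DoOnce guard reset on completion.
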(event `/Game/MyHorror/Blueprints/UseInterface.BI_Use`
  (params (hitComponent :type "PrimitiveComponent Object Reference"))
  (for (_array_element _array_index) (`self.buttons`)
    (if (== _array_element hitComponent)
      (if (not (`self.moving`))
        (bind _output (`|GetArrayItem` (`self.targets`) _array_index))
        (`/Engine/EditorBlueprintResources/StandardMacros.IsValid` _output
          (:`Is Valid`
            (`self.moveToTarget` _output)))))))

(event `moveToTarget`
  (params (targetPoint :type "TargetPoint Object Reference"))
  (set `self.moving` true)
  (`/Engine/EditorBlueprintResources/StandardMacros.DoOnce` false :!label _label
    (:`Completed`
      (bind _output_get (set `self.transform` (`self.GetTransform`)))
      (bind (_direction _tr) (`Timeline|transition`)
        (:`Update`
          (`self.K2_SetActorTransform` (`KismetMathLibrary.TLerp` _output_get (`self.GetTransform` targetPoint) _tr)))
        (:`Finished`
          (set `self.transform` (`self.GetTransform`))
          (set `self.moving` false)
          (goto _label :!via `Reset`))))))

(fn `UserConstructionScript`
  (locals (floorIndex :type Integer))
  (bind _arrow (`self.Arrow`))
  (bind _relativerotation (`SceneComponent.RelativeRotation` _arrow))
  (for _index (range 1 (+ (`KismetArrayLibrary.Array_Length` (`self.targets`)) 1))
    (set `local.floorIndex` _index)
    (bind _returnvalue (+ (* (0.0 0.0 30.0) _index) (`SceneComponent.RelativeLocation` _arrow)))
    (bind _returnvalue_2 (`AddComponent|NODE_AddStaticMeshComponent-0` :`RelativeTransform` (`KismetMathLibrary.MakeTransform` _returnvalue _relativerotation (0.2 0.2 0.2))))
    (`KismetArrayLibrary.Array_Add` (`self.buttons`) _returnvalue_2)
    (`StaticMeshComponent.SetStaticMesh` _returnvalue_2 "/Game/Geometry/Meshes/1M_Cube_Chamfer.1M_Cube_Chamfer")
    (`PrimitiveComponent.SetMaterial` _returnvalue_2 0 "/Engine/VREditor/LaserPointer/LaserPointerMaterial.LaserPointerMaterial")
    (bind _returnvalue_3 (`AddComponent|NODE_AddTextRenderComponent-0` :`RelativeTransform` (`KismetMathLibrary.MakeTransform` (+ _returnvalue (-10.0 12.0 -15.0)) _relativerotation)))
    (`TextRenderComponent.K2_SetText` _returnvalue_3 (`KismetTextLibrary.Conv_IntToText` (`local.floorIndex`)))))