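; Elevator door actor that slides open once, when the first-person character begins overlapping it while facing a qualifying direction.
; The facing test runs only at overlap start, summing the world Y components of the camera and root forward vectors and requiring zero or less.
; A DoOnce then plays a timeline that slides both doors apart along relative X, scaled by OpenWidth from positions cached in the Construction Script.
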(event `self.ReceiveActorBeginOverlap`
  (params (OtherActor :type "Actor Object Reference"))
  (bind _openwidth (`self.openWidth`))
  (bind _asfirst_person_character (cast `/Game/FirstPersonBP/Blueprints/FirstPersonCharacter` OtherActor))
  (if (<= (+ (.y (`SceneComponent.GetForwardVector` (`/Game/FirstPersonBP/Blueprints/FirstPersonCharacter.FirstPersonCamera` _asfirst_person_character))) (.y (`SceneComponent.GetForwardVector` (`self.DefaultSceneRoot`)))) 0.0)
    (`/Engine/EditorBlueprintResources/StandardMacros.DoOnce` false
      (:`Completed`
        (bind (_direction _open) (`Timeline|openDoorsTimeline` :!via `PlayFromStart`)
          (:`Update`
            (bind _returnvalue (`KismetMathLibrary.MakeVector` _open))
            (`SceneComponent.K2_SetRelativeLocation` (`self.Door1`) (+ (* _returnvalue _openwidth) (`self.door1InitLocation`)) false false)
            (`SceneComponent.K2_SetRelativeLocation` (`self.Door2`) (+ (* _returnvalue (* _openwidth -1.0)) (`self.door2InitLocation`)) false false)))))))

(fn `UserConstructionScript`
  (set `self.door1InitLocation` (`SceneComponent.RelativeLocation` (`self.Door1`)))
  (set `self.door2InitLocation` (`SceneComponent.RelativeLocation` (`self.Door2`))))