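; BP_Door is an interactable door that swings open and closed by rotating its Arrow component along a timeline.
; The use event ignores broken doors and lets a locked door move only if the player character's Keys array contains that door.
; Permitted uses alternate between playing and reversing the timeline through a FlipFlop.
; Separate OpentheDoor and CloseDoor events force either motion and set IsOpened, bypassing those checks.
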(event `/Game/MyHorror/Blueprints/UseInterface.BI_Use`
  (params (hitComponent :type "PrimitiveComponent Object Reference"))
  (if (`self.isBroken`)
    _
    (elif (`self.isLocked`)
      (bind _canbeopened (`self.canBeOpened`))
      (if _canbeopened
        (`/Engine/EditorBlueprintResources/StandardMacros.FlipFlop` :!label _label
          (:`A`
            (bind (_direction _dooropen) (`Timeline|OpenDoor` :!label _label_2)
              (:`Update`
                (`SceneComponent.K2_SetRelativeRotation` (`self.Arrow`) (`KismetMathLibrary.RLerp` (struct) (struct :`Yaw` 90.0) _dooropen) false false))))
          (:`B`
            (goto _label_2 :!via `Reverse`))))
      (else
        (goto _label)))))

(event `CloseDoor`
  (set `self.isOpened` false)
  (goto _label_2 :!via `ReverseFromEnd`))

(event `OpentheDoor`
  (set `self.isOpened` true)
  (goto _label_2 :!via `PlayFromStart`))

(fn `canBeOpened`
  (returns (canBeOpened :type Boolean))
  (bind _asfirst_person_character (cast `/Game/FirstPersonBP/Blueprints/FirstPersonCharacter` (`GameplayStatics.GetPlayerCharacter` 0)))
  (for _array_element (`/Game/FirstPersonBP/Blueprints/FirstPersonCharacter.keys` _asfirst_person_character)
    (if (== _array_element self)
      (return true)))
  (return false))

(fn `UserConstructionScript`)