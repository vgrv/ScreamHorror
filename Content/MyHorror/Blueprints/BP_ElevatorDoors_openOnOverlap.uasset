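; Elevator doors that slide open the first time the FirstPersonCharacter overlaps the actor.
; A DoOnce gate starts OpenDoorsTimeline, whose updates nudge the Arrow and Arrow1 components one unit in opposite X directions.
; The timeline acts only as a timed ticker, so travel distance depends on frame rate, and nothing closes the doors.
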(event `self.ReceiveActorBeginOverlap`
  (params (OtherActor :type "Actor Object Reference"))
  (bind _arrow (`self.Arrow`))
  (bind _arrow1 (`self.Arrow1`))
  (cast `/Game/FirstPersonBP/Blueprints/FirstPersonCharacter` OtherActor)
  (`/Engine/EditorBlueprintResources/StandardMacros.DoOnce` false
    (:`Completed`
      (`Timeline|openDoorsTimeline`
        (:`Update`
          (`SceneComponent.K2_SetRelativeLocation` _arrow (+ (`SceneComponent.RelativeLocation` _arrow) (1.0 0.0 0.0)) false false)
          (`SceneComponent.K2_SetRelativeLocation` _arrow1 (+ (`SceneComponent.RelativeLocation` _arrow1) (-1.0 0.0 0.0)) false false))))))

(fn `UserConstructionScript`)