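; Chandelier hazard actor that drops on command and kills the player on contact.
; Its three mesh parts start with physics off, and StartFalling turns simulation on for all of them.
; After a fixed delay it spawns an explosion particle effect at each part's location.
; An overlap with any part calls Death on the first-person character, whether or not the chandelier is falling.
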(event `self.ReceiveBeginPlay`
  (for _array_element (`|MakeArray` (`self.Cylinder`) (`self.StaticMesh`) (`self.StaticMesh1`))
    (`PrimitiveComponent.SetSimulatePhysics` _array_element false)))

(event `StartFalling`
  (bind _array (`|MakeArray` (`self.Cylinder`) (`self.StaticMesh`) (`self.StaticMesh1`)))
  (for _array_element _array
    (`PrimitiveComponent.SetSimulatePhysics` _array_element true))
  (`KismetSystemLibrary.Delay` 1.8)
  (for _array_element_2 _array
    (`GameplayStatics.SpawnEmitterAtLocation` "/Game/StarterContent/Particles/P_Explosion.P_Explosion" (`SceneComponent.K2_GetComponentLocation` _array_element_2))))

(event `self.StaticMesh1.OnComponentBeginOverlap`
  (params (OverlappedComponent :type "PrimitiveComponent Object Reference") (OtherActor :type "Actor Object Reference") (OtherComp :type "PrimitiveComponent Object Reference") (OtherBodyIndex :type Integer) (bFromSweep :type Boolean) (SweepResult :type "HitResult Structure (by ref)"))
  (bind _asfirst_person_character (cast `/Game/FirstPersonBP/Blueprints/FirstPersonCharacter` OtherActor))
  (`/Game/FirstPersonBP/Blueprints/FirstPersonCharacter.Death` _asfirst_person_character))

(event `self.StaticMesh.OnComponentBeginOverlap`
  (params (OverlappedComponent :type "PrimitiveComponent Object Reference") (OtherActor :type "Actor Object Reference") (OtherComp :type "PrimitiveComponent Object Reference") (OtherBodyIndex :type Integer) (bFromSweep :type Boolean) (SweepResult :type "HitResult Structure (by ref)"))
  (bind _asfirst_person_character (cast `/Game/FirstPersonBP/Blueprints/FirstPersonCharacter` OtherActor))
  (`/Game/FirstPersonBP/Blueprints/FirstPersonCharacter.Death` _asfirst_person_character))

(event `self.Cylinder.OnComponentBeginOverlap`
  (params (OverlappedComponent :type "PrimitiveComponent Object Reference") (OtherActor :type "Actor Object Reference") (OtherComp :type "PrimitiveComponent Object Reference") (OtherBodyIndex :type Integer) (bFromSweep :type Boolean) (SweepResult :type "HitResult Structure (by ref)"))
  (bind _asfirst_person_character (cast `/Game/FirstPersonBP/Blueprints/FirstPersonCharacter` OtherActor))
  (`/Game/FirstPersonBP/Blueprints/FirstPersonCharacter.Death` _asfirst_person_character))

(fn `UserConstructionScript`)