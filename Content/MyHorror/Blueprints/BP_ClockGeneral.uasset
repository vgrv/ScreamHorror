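; Clock actor that shows a time by rotating its hour and minute hands from the Hours and Minutes variables.
; On BeginPlay it sets the starting time and, if RotationSpeed is non-zero, starts a looping timer firing RotationSpeed times per second.
; Each tick of that timer runs forward1Minute, which advances and wraps the counters, then calls setTime to set each hand's relative yaw.
; The hour hand jumps in whole-hour steps.
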(event `self.ReceiveBeginPlay`
  (`self.setTime` (`self.Hours`) (`self.Minutes`))
  (if (!= (`self.rotationSpeed`) 0.0)
    (`KismetSystemLibrary.K2_SetTimer` null "forward1Minute" (/ 1.0 (`self.rotationSpeed`)) true)))

(event `setTime`
  (params (`Hours (1-12)` :type Integer) (`Minutes (0-59)` :type Integer))
  (`SceneComponent.K2_SetRelativeRotation` (`self.HoursHandScene`) (`KismetMathLibrary.MakeRotator` 0.0 0.0 (* (/ (`KismetMathLibrary.Conv_IntToDouble` (mod `Hours (1-12)` 12)) 12.0) 360.0)) false false)
  (`SceneComponent.K2_SetRelativeRotation` (`self.MinsHandScene`) (`KismetMathLibrary.MakeRotator` 0.0 0.0 (* (/ (`KismetMathLibrary.Conv_IntToDouble` (mod `Minutes (0-59)` 60)) 60.0) 360.0)) false false))

(fn `forward1Minute`
  (if (>= (`self.Minutes`) 60)
    (set `self.Minutes` 0)
    (set `self.Hours` (+ (`self.Hours`) 1))
    (else
      (set `self.Minutes` (+ (`self.Minutes`) 1))))
  (if (>= (`self.Hours`) 12)
    (set `self.Hours` 0))
  (`self.setTime` (`self.Hours`) (`self.Minutes`)))

(fn `UserConstructionScript`)