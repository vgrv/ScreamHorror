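; BP_WatchFace is a Blueprint that lays out the numbers 1 to 12 in a ring to form a watch face.
; The construction script adds a text render component per number, placing it at 30-degree steps on a circle in the local XY plane using sine, cosine and Radius.
; Each label is rotated to lie flat and uses a translucent text material.
; The event graph holds no active logic.
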(fn `UserConstructionScript`
  (bind _radius (`self.radius`))
  (for _index (range 1 13)
    (bind _returnvalue (* (`KismetMathLibrary.Conv_IntToDouble` _index) 30.0))
    (bind _returnvalue_2 (`AddComponent|NODE_AddTextRenderComponent-0` :`RelativeTransform` (`KismetMathLibrary.MakeTransform` (`KismetMathLibrary.MakeVector` (* (`KismetMathLibrary.DegCos` _returnvalue) _radius) (* _radius (`KismetMathLibrary.DegSin` _returnvalue)) 0.0) (struct :`Pitch` 90.0 :`Yaw` 180.0))))
    (`TextRenderComponent.K2_SetText` _returnvalue_2 (`KismetTextLibrary.Conv_IntToText` _index))
    (`PrimitiveComponent.SetMaterial` _returnvalue_2 0 "/Engine/EngineMaterials/DefaultTextMaterialTranslucent.DefaultTextMaterialTranslucent")))