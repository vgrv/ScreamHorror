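; BP_Key is a key pickup that gives the player access entries for the doors it lists.
; On the BIUse event, it casts player 0 to FirstPersonCharacter and checks each Doors entry against that character's Keys array.
; A missing entry is added to Keys, then a message prints and the key destroys itself.
; The IsKeyInInventory flag is never reset, so one match blocks every later entry in the loop.
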(event `/Game/MyHorror/Blueprints/UseInterface.BI_Use`
  (params (hitComponent :type "PrimitiveComponent Object Reference"))
  (bind _asfirst_person_character (cast `/Game/FirstPersonBP/Blueprints/FirstPersonCharacter` (`GameplayStatics.GetPlayerCharacter` 0)))
  (for _array_element (`self.doors`)
    (bind _keys (`/Game/FirstPersonBP/Blueprints/FirstPersonCharacter.keys` _asfirst_person_character))
    (for _array_element_2 _keys
      (if (== _array_element_2 _array_element)
        (set `self.isKeyInInventory` true)
        (break)))
    (if (not (`self.isKeyInInventory`))
      (`KismetArrayLibrary.Array_Add` _keys _array_element)
      (`KismetSystemLibrary.PrintString` "Got a new key!")
      (`self.K2_DestroyActor`))))

(fn `UserConstructionScript`)